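; Player character with weapon handling, dialogue interaction, footstep noise and a toggleable camera vision mode.
; Reload, draw and holster montages set an upper-body flag, with notifies driving WeaponSystem equips and completion chaining slot swaps.
; Separate pickup functions manage primary and secondary guns on hold and stowed sockets.
; Footsteps report movement-scaled noise with a particle indicator, while camera vision drives a material parameter collection and spotlight through a timeline.
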(event `InputAction|Dialouge`
  (params (Key :type "Key Structure"))
  (:`Pressed`
    (if (`PrimitiveComponent.IsOverlappingActor` (`self.CapsuleComponent`) (stale `self.ReceiveActorBeginOverlap` _asbp_dialouge))
      (`/Game/WeaponSystem/Dialouge/BP_Dialouge.InteractionEvent` (stale `self.ReceiveActorBeginOverlap` _asbp_dialouge) self "WeaponNone"))))

(event `self.ReceiveActorBeginOverlap`
  (params (OtherActor :type "Actor Object Reference"))
  (bind _asbp_dialouge (cast `/Game/WeaponSystem/Dialouge/BP_Dialouge` OtherActor)))

(event `SetcharacterMovementMode_1`
  (params (Movement :type "EMovementMode Enum" :default "MOVE_None"))
  (`CharacterMovementComponent.SetMovementMode` (`self.CharacterMovement`) Movement 0))

(event `Foots`
  (bind _walksoundrange (`self.WalkSoundRange`))
  (bind _runsoundrange (`self.RunSoundRange`))
  (bind _returnvalue (/ _runsoundrange 50.0))
  (bind _returnvalue_2 (/ _walksoundrange 50.0))
  (switch `/Game/WeaponSystem/Player/Custom_Me/PADong/EPlayerMoveMent` (`self.Movement`)
    (:`NewEnumerator0`
      (`self.ReportNoise` (`KismetMathLibrary.MakeVector` _returnvalue_2 _returnvalue_2) (struct :`R` 1.0 :`G` 0.102237 :`B` 0.07239 :`A` 1.0) _walksoundrange))
    (:`NewEnumerator2`
      (`self.ReportNoise` (`KismetMathLibrary.MakeVector` _returnvalue _returnvalue) (struct :`R` 1.0 :`G` 0.102237 :`B` 0.07239 :`A` 1.0) _runsoundrange))))

(event `InputAction|Fever_Camera`
  (params (Key :type "Key Structure"))
  (:`Pressed`
    (`/Engine/EditorBlueprintResources/StandardMacros.FlipFlop`
      (:`A`
        (set `self.TemCamerOn?` true)
        (bind (_direction _depth _cameradistance _alpha) (`Timeline|타임라인_1` :!label _label)
          (:`Update`
            (`KismetMaterialLibrary.SetScalarParameterValue` "/Game/Effect/ScreenEffects/Materials/MPC_DataPP.MPC_DataPP" "Depth" _depth)
            (`KismetMaterialLibrary.SetScalarParameterValue` "/Game/Effect/ScreenEffects/Materials/MPC_DataPP.MPC_DataPP" "Alpha" _alpha)
            (if (`self.TemCamerOn?`)
              (`KismetSystemLibrary.Delay` 1.0)
              (`SceneComponent.SetHiddenInGame` (`self.SpotLight`) false false)
              (else
                (`SceneComponent.SetHiddenInGame` (`self.SpotLight`) true false))))))
      (:`B`
        (set `self.TemCamerOn?` false)
        (goto _label :!via `Reverse`)))))

(event `self.K2_PlayReloadAnimation`
  (bind _mesh (`self.Mesh`))
  (set `self.UpperBody?` true)
  (switch `EWeaponType` (`GunBase.WeaponType` (`WeaponComponent.CurrentEquipWeapon` (`self.WeaponSystem`)))
    (:`Pistol`
      (`|PlayMontage` _mesh "/Game/WeaponSystem/Player/UsePlayerAnim/Retarget2/RE2_RE_AM_PistolReload.RE2_RE_AM_PistolReload" 1.2
        (:`OnCompleted`
          _)))
    (:`AssultRifle`
      (`|PlayMontage` _mesh "/Game/WeaponSystem/Player/UsePlayerAnim/Retarget2/RE2_RE_AM_RifleReload1.RE2_RE_AM_RifleReload1" 1.2 :!label _label_2
        (:`OnCompleted`
          _)))
    (:`SniperRifle`
      (goto _label_2)))
  (`WeaponComponent.ReloadAnimationComplete` (`self.WeaponSystem`))
  (set `self.UpperBody?` false))

(event `self.K2_PlaySlotReleaseAnimation`
  (params (_Slot :type "EWeaponSlot Enum" :default "WeaponNone"))
  (bind _mesh (`self.Mesh`))
  (bind _mesh_2 (`self.Mesh`))
  (switch `EWeaponSlot` (`WeaponComponent.CurrentGunSlot` (`self.WeaponSystem`))
    (:`WeaponNone`
      (switch `EWeaponSlot` _Slot :!label _label_3
        (:`WeaponSlot1`
          (set `self.UpperBody?` true)
          (`|PlayMontage` _mesh_2 "/Game/WeaponSystem/Player/UsePlayerAnim/Retarget2/RE2_RE_Slot1_TakeUp.RE2_RE_Slot1_TakeUp"
            (:`OnCompleted`
              (set `self.UpperBody?` false))
            (:`OnNotifyBegin`
              (`WeaponComponent.EquipWeapon` (`self.WeaponSystem`) _Slot :!label _label_4))))
        (:`WeaponSlot2`
          (set `self.UpperBody?` true)
          (`|PlayMontage` _mesh_2 "/Game/WeaponSystem/Player/UsePlayerAnim/Retarget2/RE2_RE_Rifle03_TakeUp.RE2_RE_Rifle03_TakeUp"
            (:`OnCompleted`
              (set `self.UpperBody?` false))
            (:`OnNotifyBegin`
              (goto _label_4))))))
    (:`WeaponSlot1`
      (set `self.UpperBody?` true)
      (`|PlayMontage` _mesh "/Game/WeaponSystem/Player/UsePlayerAnim/Retarget2/RE2_RE_slot01_hidedown1.RE2_RE_slot01_hidedown1"
        (:`OnCompleted`
          (set `self.UpperBody?` false)
          (goto _label_3))
        (:`OnNotifyBegin`
          (`WeaponComponent.EquipWeapon` (`self.WeaponSystem`) "WeaponNone" :!label _label_5))))
    (:`WeaponSlot2`
      (set `self.UpperBody?` true)
      (`|PlayMontage` _mesh "/Game/WeaponSystem/Player/UsePlayerAnim/Retarget2/RE2_RE_slot2_hideup.RE2_RE_slot2_hideup"
        (:`OnCompleted`
          (set `self.UpperBody?` false)
          (goto _label_3))
        (:`OnNotifyBegin`
          (goto _label_5))))))

(event `self.K2_PlaySlotHoldAnimation`
  (params (_Slot :type "EWeaponSlot Enum" :default "WeaponNone"))
  (bind _mesh (`self.Mesh`))
  (switch `EWeaponSlot` _Slot
    (:`WeaponSlot1`
      (set `self.UpperBody?` true)
      (`|PlayMontage` _mesh "/Game/WeaponSystem/Player/UsePlayerAnim/Retarget2/RE2_RE_slot01_hidedown1.RE2_RE_slot01_hidedown1"
        (:`OnCompleted`
          (set `self.UpperBody?` false))
        (:`OnNotifyBegin`
          (`WeaponComponent.EquipWeapon` (`self.WeaponSystem`) "WeaponNone" :!label _label_6))))
    (:`WeaponSlot2`
      (set `self.UpperBody?` true :!label _label_7)
      (`|PlayMontage` _mesh "/Game/WeaponSystem/Player/UsePlayerAnim/Retarget2/RE2_RE_slot2_hideup.RE2_RE_slot2_hideup"
        (:`OnCompleted`
          (set `self.UpperBody?` false))
        (:`OnNotifyBegin`
          (goto _label_6))))
    (:`WeaponSlot3`
      (goto _label_7))))

(fn `Get Center Of Crosshair Location`
  (returns (IsHit :type Boolean) (Location :type "Vector Structure"))
  (return false (0.0 0.0 0.0)))

(fn `PickUp Gun`
  (params (NewGun :type "/Game/WeaponSystem/Item/Guns/BP_Gun Object Reference"))
  (`/Engine/EditorBlueprintResources/StandardMacros.IsValid` (`self.PrimaryGun`)
    (:`Is Valid`
      (`/Engine/EditorBlueprintResources/StandardMacros.IsValid` (`self.SecondaryGun`)
        (:`Is Valid`
          (bind _returnvalue (`self.EquippedGun`)
            (:`Is Valid`
              (`self.K2_DetachFromActor` _returnvalue "KeepWorld" "KeepWorld" "KeepWorld")
              (`/Game/WeaponSystem/Item/Guns/BP_Gun.DropGun` _returnvalue)
              (`self.SetEquippedGun` null)
              (`self.PickUp Gun` (`local.NewGun`)))))
        (:`Is Not Valid`
          (set `self.SecondaryGun` (`local.NewGun`))
          (`self.UpdateGunAttachments` :!label _label)
          (`self.SetOwner` (`local.NewGun`) self))))
    (:`Is Not Valid`
      (set `self.PrimaryGun` (`local.NewGun`))
      (goto _label))))

(fn `ReportNoise`
  (params (Size :type "Vector Structure") (Color :type "LinearColor Structure") (Range :type "Float (double-precision)"))
  (bind _particlesystem (`self.ParticleSystem`))
  (`AISense_Hearing.ReportNoiseEvent` (`self.K2_GetActorLocation`) 1.0 self Range)
  (`ActorComponent.Activate` _particlesystem true)
  (`FXSystemComponent.SetVectorParameter` _particlesystem "Size" Size)
  (`FXSystemComponent.SetColorParameter` _particlesystem "Color" Color))

(fn `UpdateGunAttachments`
  (`|ExecutionSequence`
    (:`then_0`
      (bind _returnvalue (`self.EquippedGun`)
        (:`Is Valid`
          (set `/Game/WeaponSystem/Item/Guns/BP_Gun.canShoot` false _returnvalue)
          (`self.K2_AttachToComponent` _returnvalue (`self.Mesh`) "GunHoldSocket" "SnapToTarget" "SnapToTarget" "SnapToTarget" true))))
    (:`then_1`
      (bind _returnvalue_2 (`self.StowedGun`)
        (:`Is Valid`
          (set `/Game/WeaponSystem/Item/Guns/BP_Gun.canShoot` false _returnvalue_2)
          (`self.K2_AttachToComponent` _returnvalue_2 (`self.Mesh`) "GunStowedSocket" "SnapToTarget" "SnapToTarget" "SnapToTarget" true))))))

(fn `UserConstructionScript`
  (`SkinnedMeshComponent.SetLeaderPoseComponent` (`self.Head`) (`self.Mesh`) false false)
  (`parent.UserConstructionScript`))