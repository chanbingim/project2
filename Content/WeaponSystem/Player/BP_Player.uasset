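; Third-person player character with gun handling, camera modes and footstep noise for AI perception.
; Primary and secondary gun slots feed socket attachment, selector switching and firing, which requires aiming.
; Timelines drive aim zoom, shoulder swapping and a search-vision toggle that sets post-process depth and boom length.
; Footsteps report noise ranged by walk, crouch or run, shown by a sized, colored effect; pickup and interaction are unfinished stubs.
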(event `InputAction|Switch Selecter`
  (params (Key :type "Key Structure"))
  (:`Pressed`
    (bind _returnvalue (`self.EquippedGun`)
      (:`Is Valid`
        (`/Game/WeaponSystem/Item/Guns/BP_Gun.Switch Selector` _returnvalue)))))

(event `Key|RightMouseButton`
  (params (Key :type "Key Structure"))
  (:`Pressed`
    (if (`self.Is_Zoom`)
      (`|ExecutionSequence`
        (:`then_0`
          (`self.EquippedGun`
            (:`Is Valid`
              (set `self.AimButtonDown` true))))
        (:`then_1`
          (bind (_direction _fov _front_cam) (`Timeline|Zoom_Camera` :!label _label)
            (:`Update`
              (`CameraComponent.SetFieldOfView` (`self.FollowCamera`) _fov)
              (set `SpringArmComponent.TargetArmLength` _front_cam (`self.CameraBoom`))))))
      (else
        (`|ExecutionSequence` :!label _label_2
          (:`then_0`
            (goto _label :!via `Reverse`))
          (:`then_1`
            (set `self.AimButtonDown` false)
            (set `self.TemCamer_On?` false)))))))

(event `Key|LeftShift`
  (params (Key :type "Key Structure"))
  (:`Pressed`
    (goto _label_2)))

(event `InputAction|Camera_LeftMove`
  (params (Key :type "Key Structure"))
  (:`Pressed`
    (set `self.Change_Left` true)
    (bind (_direction _move_distance) (`Timeline|Wibing_Cam` :!label _label_3)
      (:`Update`
        (`SceneComponent.K2_SetWorldLocation` (`self.FollowCamera`) (+ (`SceneComponent.K2_GetComponentLocation` (`self.LeftCamera`)) (* _move_distance (`self.GetActorRightVector`)) (* (`self.GetActorUpVector`) 60.0)) false false)))))

(event `InputAction|Camera_RightMove`
  (params (Key :type "Key Structure"))
  (:`Pressed`
    (set `self.Change_Left` false)
    (goto _label_3 :!via `Reverse`)))

(event `InputAction|Fire`
  (params (Key :type "Key Structure"))
  (:`Pressed`
    (if (`self.AimButtonDown`)
      (bind _returnvalue (`self.EquippedGun`)
        (:`Is Valid`
          (`/Game/WeaponSystem/Item/Guns/BP_Gun.Fire` _returnvalue (`self.FollowCamera`))))))
  (:`Released`
    (bind _returnvalue_2 (`self.EquippedGun`)
      (:`Is Valid`
        (`/Game/WeaponSystem/Item/Guns/BP_Gun.Release Fire` _returnvalue_2)))))

(event `self.CapsuleComponent.OnComponentBeginOverlap`
  (params (OverlappedComponent :type "PrimitiveComponent Object Reference") (OtherActor :type "Actor Object Reference") (OtherComp :type "PrimitiveComponent Object Reference") (OtherBodyIndex :type Integer) (bFromSweep :type Boolean) (SweepResult :type "HitResult Structure (by ref)"))
  (if (`KismetSystemLibrary.DoesImplementInterface` OtherActor)
    _))

(event `self.CapsuleComponent.OnComponentEndOverlap`
  (params (OverlappedComponent :type "PrimitiveComponent Object Reference") (OtherActor :type "Actor Object Reference") (OtherComp :type "PrimitiveComponent Object Reference") (OtherBodyIndex :type Integer))
  (if (`KismetSystemLibrary.DoesImplementInterface` OtherActor)
    _))

(event `InputAction|Interract`
  (params (Key :type "Key Structure"))
  (:`Pressed`
    (for _array_element (`PrimitiveComponent.GetOverlappingActors` (`self.CapsuleComponent`) null)
      (if (`KismetSystemLibrary.DoesImplementInterface` _array_element)
        _))))

(event `InputAction|Jump`
  (params (Key :type "Key Structure"))
  (:`Pressed`
    (message `/Game/Model/ProjectAnimation/Bp_PlayerMo.GetJumping` (`SkeletalMeshComponent.GetAnimInstance` (`self.Mesh`)))))

(event `Player_Jump`
  (`self.Jump`))

(event `Foots`
  (bind _walk_sound (`self.Walk_Sound`))
  (bind _crouch_sound (`self.Crouch_Sound`))
  (bind _run_sound (`self.Run_Sound`))
  (bind _returnvalue (/ _run_sound 50.0))
  (bind _returnvalue_2 (/ _walk_sound 50.0))
  (bind _returnvalue_3 (/ _crouch_sound 50.0))
  (switch `/Game/WeaponSystem/Player/Custom_Me/PADong/EPlayerMoveMent` (`self.Movement`)
    (:`NewEnumerator0`
      (`self.NewMacro` :!label _label_4
        (:`Walk_then`
          (`self.ReportNoise` (`KismetMathLibrary.MakeVector` _returnvalue_2 _returnvalue_2) (struct :`R` 1.0 :`G` 0.701951 :`A` 1.0) _walk_sound))
        (:`Crouch_then`
          (`self.ReportNoise` (`KismetMathLibrary.MakeVector` _returnvalue_3 _returnvalue_3) (struct :`R` 0.043873 :`G` 0.062315 :`B` 0.270833 :`A` 1.0) _crouch_sound))
        (:`Run_then`
          (`self.ReportNoise` (`KismetMathLibrary.MakeVector` _returnvalue _returnvalue) (struct :`R` 1.0 :`G` 0.030746 :`B` 0.060593 :`A` 1.0) _run_sound))))
    (:`NewEnumerator1`
      (goto _label_4 :!via `Crouch`))
    (:`NewEnumerator2`
      (goto _label_4 :!via `Run`))))

(event `/Game/Model/ProjectAnimation/Bp_PlayerMo.SetcharacterMovementMode`
  (params (Movement :type "EMovementMode Enum" :default "MOVE_None"))
  (`CharacterMovementComponent.SetMovementMode` (`self.CharacterMovement`) Movement 0))

(event `InputAction|Fever_Camera`
  (params (Key :type "Key Structure"))
  (:`Pressed`
    (`/Engine/EditorBlueprintResources/StandardMacros.FlipFlop`
      (:`A`
        (set `self.TemCamer_On?` true)
        (bind (_direction _customdepth _cameramove) (`Timeline|Search_Ai` :!label _label_5)
          (:`Update`
            (`KismetMaterialLibrary.SetScalarParameterValue` "/Game/WeaponSystem/Player/Custom_Me/Fever/PPE_Under.PPE_Under" "Depth" _customdepth)
            (`self.WorldLocation_SearchAI` _cameramove))))
      (:`B`
        (set `self.TemCamer_On?` false)
        (goto _label_5 :!via `Reverse`)))))

(event `Key|LeftShift`
  (params (Key :type "Key Structure"))
  (:`Pressed`
    (goto _label_5 :!via `Reverse`)))

(fn `GetMomentInput`
  (returns (Speed :type "Float (double-precision)"))
  (return (`self.GetInputAxisValue`)))

(fn `PickUp Gun`
  (params (NewGun :type "/Game/WeaponSystem/Item/Guns/BP_Gun Object Reference")))

(fn `ReportNoise`
  (params (EffectSize :type "Vector Structure") (EffectColor :type "LinearColor Structure") (EffectRange :type "Float (double-precision)"))
  (bind _noiserangeeffect (`self.NoiseRangeEffect`))
  (`AISense_Hearing.ReportNoiseEvent` (`self.K2_GetActorLocation`) 1.0 self EffectRange)
  (`ActorComponent.Activate` _noiserangeeffect true)
  (`FXSystemComponent.SetVectorParameter` _noiserangeeffect "Size" EffectSize)
  (`FXSystemComponent.SetColorParameter` _noiserangeeffect "Color" EffectColor)
  (`KismetSystemLibrary.PrintString` (`KismetStringLibrary.Conv_VectorToString` EffectSize))
  (`KismetSystemLibrary.PrintString` (`KismetStringLibrary.Conv_ColorToString` EffectColor))
  (return))

(fn `UpdateGunAttachments`
  (`|ExecutionSequence`
    (:`then_0`
      (bind _returnvalue (`self.EquippedGun`)
        (:`Is Valid`
          (`self.K2_AttachToComponent` _returnvalue (`self.Mesh`) "GunHoldSocket" "SnapToTarget" "SnapToTarget" "SnapToTarget" true))))
    (:`then_1`
      (bind _returnvalue_2 (`self.StowedGun`)
        (:`Is Valid`
          (`self.K2_AttachToComponent` _returnvalue_2 (`self.Mesh`) "GunStowedSocket" "SnapToTarget" "SnapToTarget" "SnapToTarget" true))))))

(fn `UserConstructionScript`
  (`parent.UserConstructionScript`))

(fn `WorldLocation_SearchAI`
  (params (A :type "Float (single-precision)"))
  (returns (ReturnValue :type "Float (double-precision)"))
  (bind _output_get (set `SpringArmComponent.TargetArmLength` A (`self.CameraBoom`)))
  (return _output_get))