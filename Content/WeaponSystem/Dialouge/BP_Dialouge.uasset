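; Dialogue actor that shows chained subtitle lines with voice audio, triggered once by player overlap or through an interaction event.
; Lines load from DT_TextTable, each advancing to its next row after the sound's duration plus a short delay.
; Interaction also snaps the player to the skeletal mesh, plays a seated typing montage with weapon unequipped, then re-equips it.
; Leaving the trigger removes the widget when the current row allows skipping.
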(event `self.ReceiveBeginPlay`
  (`self.LoadData`))

(event `LoadData`
  (bind (_texttable_level _texttable_text _texttable_sound _texttable_next_text) (break `/Game/WeaponSystem/Dialouge/ST_Text` (`self.TextTable`)))
  (bind _returnvalue (`|GetDataTableRow` "/Game/WeaponSystem/Dialouge/DT_TextTable.DT_TextTable" (`self.TextID`))
    (:`then`
      (set `self.TextTable` _returnvalue)
      (set `self.Text` _texttable_text)
      (set `self.Sound` _texttable_sound)
      (set `self.NextTextID` _texttable_next_text))
    (:`RowNotFound`
      (`KismetSystemLibrary.PrintString` "Not Found Text "))))

(event `self.ReceiveActorBeginOverlap`
  (params (OtherActor :type "Actor Object Reference"))
  (if (and (== (`self.GetOwner` OtherActor) (`GameplayStatics.GetPlayerController` 0)) (not (`self.BoxStatus`)) (`|EnumEquality` (`self.TriggerType`) "NewEnumerator0"))
    (set `self.BoxStatus` true)
    (bind _returnvalue (`|CreateWidget` "/Game/WeaponSystem/Dialouge/WBI_Text.WBI_Text_C"))
    (bind _output_get (set `self.TextUI` _returnvalue))
    (`UserWidget.AddToViewport` _output_get 0)
    (`self.PrintText`)))

(event `PrintText`
  (bind _nexttextid (`self.NextTextID`))
  (`TextBlock.SetText` (`/Game/WeaponSystem/Dialouge/WBI_Text.TextLog` (`self.TextUI`)) (`self.Text`))
  (`GameplayStatics.PlaySoundAtLocation` (`self.Sound`) (`self.K2_GetActorLocation` (`self.GetOwner` (`GameplayStatics.GetPlayerController` 0))) (struct) 1.0 1.0 0.0 null null null null)
  (`KismetSystemLibrary.Delay` (+ (`SoundBase.Duration` (`self.Sound`)) 0.3))
  (if (!= _nexttextid "None")
    (set `self.TextID` _nexttextid)
    (`self.LoadData`)
    (`self.PrintText`)
    (else
      (`self.Remove`))))

(event `Remove`
  (`Widget.RemoveFromParent` (`self.TextUI`))
  (message `AudioLinkBlueprintInterface.StopLink` (`self.Sound`)))

(event `self.ReceiveActorEndOverlap`
  (params (OtherActor :type "Actor Object Reference"))
  (bind (_texttable_level _texttable_text _texttable_sound _texttable_next_text _texttable_delay _texttable_skip) (break `/Game/WeaponSystem/Dialouge/ST_Text` (`self.TextTable`)))
  (if (== (`self.GetOwner` OtherActor) (`GameplayStatics.GetPlayerController` 0))
    (if _texttable_skip
      (`self.Remove`))))

(event `InteractionEvent`
  (params (Player :type "/Game/WeaponSystem/Player/BP_Player2 Object Reference") (WeaponSlot :type "EWeaponSlot Enum" :default "WeaponNone"))
  (set `self.BoxStatus` true)
  (`self.K2_SetActorLocation` Player (`SceneComponent.K2_GetComponentLocation` (`self.SkeletalMesh`)) false false)
  (bind _returnvalue (`|CreateWidget` "/Game/WeaponSystem/Dialouge/WBI_Text.WBI_Text_C"))
  (bind _output_get (set `self.TextUI` _returnvalue))
  (`UserWidget.AddToViewport` _output_get 0)
  (`self.InteractionPrint`)
  (set `/Game/WeaponSystem/Player/BP_Player2.UpperBody?` true Player)
  (if (`MyCharacter.Is_crouch` Player)
    (set `MyCharacter.Is_crouch` false Player))
  (`WeaponComponent.EquipWeapon` (`MyCharacter.WeaponSystem` Player) "WeaponNone")
  (`|PlayMontage` (`Character.Mesh` Player) "/Game/WeaponSystem/Player/UsePlayerAnim/Retarget2/RE2_48_Sitting_Typing_01_MaleA_Montage.RE2_48_Sitting_Typing_01_MaleA_Montage"
    (:`OnCompleted`
      (set `/Game/WeaponSystem/Player/BP_Player2.UpperBody?` true Player)
      (`WeaponComponent.EquipWeapon` (`MyCharacter.WeaponSystem` Player) WeaponSlot))))

(event `InteractionPrint`
  (bind _nexttextid (`self.NextTextID`))
  (`TextBlock.SetText` (`/Game/WeaponSystem/Dialouge/WBI_Text.TextLog` (`self.TextUI`)) (`self.Text`))
  (`GameplayStatics.PlaySoundAtLocation` (`self.Sound`) (`self.K2_GetActorLocation` (stale `InteractionEvent` Player)) (struct) 1.0 1.0 0.0 null null null null)
  (`KismetSystemLibrary.Delay` (+ (`SoundBase.Duration` (`self.Sound`)) 0.3))
  (if (!= _nexttextid "None")
    (set `self.TextID` _nexttextid)
    (`self.LoadData`)
    (`self.InteractionPrint`)
    (else
      (`self.Remove`))))

(fn `UserConstructionScript`)