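; Base projectile actor for weapon bullets, with material penetration and debug-line trails colored by speed relative to initial speed.
; On fast bounces, recursive reverse sphere traces find an exit point through the hit actor and any adjoining objects.
; GetNewSpeed is meant to derive exit speed from energy lost over penetration depth.
; A positive result spawns a replacement bullet at the exit; failed penetration destroys the bullet, while slower impacts keep bouncing.
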(event `self.ReceiveTick`
  (params (DeltaSeconds :type "Float (single-precision)"))
  (bind _returnvalue (`self.K2_GetActorLocation`))
  (`KismetSystemLibrary.DrawDebugLine` (`self.LastPosition`) _returnvalue (`self.GetTraceColor` (`MovementComponent.Velocity` (`self.ProjectileMovement`))) (`self.TraceDuration`))
  (set `self.LastPosition` _returnvalue))

(event `self.ProjectileMovement.OnProjectileBounce`
  (params (ImpactResult :type "HitResult Structure (by ref)") (ImpactVelocity :type "Vector Structure (by ref)"))
  (bind (_bblockinghit _binitialoverlap _time _distance _location) (`GameplayStatics.BreakHitResult` ImpactResult))
  (`KismetSystemLibrary.DrawDebugLine` (`self.LastPosition`) _location (`self.GetTraceColor` ImpactVelocity) (`self.TraceDuration`))
  (set `self.LastPosition` _location)
  ;[1 1 1] 관통 여부 확인
  (if (> (`KismetMathLibrary.VSize` ImpactVelocity) 15000.0)
    (bind (_exit_location _resultfound) (`self.ComputeExitLocation` ImpactResult ImpactVelocity))
    (if _resultfound
      (bind _new_speed (`self.GetNewSpeed` ImpactResult _exit_location ImpactVelocity))
      ;[1 1 1] 새로운 속도 구하기
      (if (> _new_speed 0.0)
        (bind _returnvalue (`|SpawnActorFromClass` "BP_BulletBase_C" (`KismetMathLibrary.MakeTransform` _exit_location) "Undefined" "OverrideRootScale" (`self.GetOwner`) null))
        (set `MovementComponent.Velocity` (* ImpactVelocity (mod _new_speed (`KismetMathLibrary.VSize` ImpactVelocity))) (`/Game/WeaponSystem/Item/Bullets/BP_BulletBase.ProjectileMovement` _returnvalue))
        (`self.K2_DestroyActor`)
        (else
          (`self.K2_DestroyActor` :!label _label)))
      (else
        (goto _label)))))

(fn `ComputeExitLocation`
  (params (HitResult :type "HitResult Structure") (ImpactVelocity :type "Vector Structure"))
  (returns (`Exit Location` :type "Vector Structure") (ResultFound :type Boolean))
  (bind _returnvalue (`KismetMathLibrary.Normal` ImpactVelocity))
  (bind (_bblockinghit _binitialoverlap _time _distance _location _impactpoint _normal _impactnormal _physmat _hitactor) (`GameplayStatics.BreakHitResult` HitResult))
  (bind _array (`|MakeArray` "ObjectTypeQuery1" "ObjectTypeQuery2" "ObjectTypeQuery3" "ObjectTypeQuery4" "ObjectTypeQuery6" :!type "EObjectTypeQuery Enum"))
  (bind (_outhits _returnvalue_2) (`KismetSystemLibrary.SphereTraceMultiForObjects` (+ (* _returnvalue 500.0) _location) _location (`SphereComponent.SphereRadius` (`self.Sphere`)) _array))
  (if _returnvalue_2
    (bind _returnvalue_3 (`KismetArrayLibrary.Array_LastIndex` _outhits))
    (for _index (range (+ _returnvalue_3 1))
      (bind (_bblockinghit_2 _binitialoverlap_2 _time_2 _distance_2 _location_2 _impactpoint_2 _normal_2 _impactnormal_2 _physmat_2 _hitactor_2) (`GameplayStatics.BreakHitResult` (`|GetArrayItem` _outhits (- _returnvalue_3 _index))))
      (if (== _hitactor_2 _hitactor)
        ;[1 1 1] 나가는 위치에 충돌 체크
        (bind (_outhit _returnvalue_4) (`KismetSystemLibrary.SphereTraceSingleForObjects` _location_2 (+ _returnvalue _location_2) (`SphereComponent.SphereRadius` (`self.Sphere`)) _array false (`|MakeArray` _hitactor)))
        (if _returnvalue_4
          (bind (_exit_location _resultfound) (`self.ComputeExitLocation` _outhit ImpactVelocity))
          (if _resultfound
            (return _exit_location true)
            (else
              (return (0.0 0.0 0.0) false) ; 결과를 찾을 수 없음
            ))
          (else
            (return _location_2 true))))))
  (return (0.0 0.0 0.0) false) ; 결과를 찾을 수 없음
)

(fn `GetNewSpeed`
  (params (Hit :type "HitResult Structure") (`Exit Location` :type "Vector Structure") (`Impact Velocity` :type "Vector Structure"))
  (returns (`New Speed` :type "Float (double-precision)"))
  (return (`KismetMathLibrary.Sqrt` (mod (- (* 0.0 (`self.Mass`) (`KismetMathLibrary.VSizeSquared` `Impact Velocity`)) (* (`KismetMathLibrary.VSize` (- `Exit Location` (`.Location` (`GameplayStatics.BreakHitResult` Hit)))) 30000.0)) (* 0.5 (`self.Mass`))))))

(fn `GetTraceColor`
  (params (Velocity :type "Vector Structure"))
  (returns (Color :type "LinearColor Structure"))
  (bind _returnvalue (mod (`KismetMathLibrary.VSize` Velocity) (`ProjectileMovementComponent.InitialSpeed` (`self.ProjectileMovement`))))
  (if (> _returnvalue 0.75)
    (return (`KismetMathLibrary.LinearColorLerp` (struct :`R` 1.0 :`G` 1.0 :`A` 1.0) (struct :`R` 1.0 :`A` 1.0) (* (- _returnvalue 0.75) 4.0)))
    (elif (> _returnvalue 0.5)
      (return (`KismetMathLibrary.LinearColorLerp` (struct :`G` 1.0 :`A` 1.0) (struct :`R` 1.0 :`G` 1.0 :`A` 1.0) (* (- _returnvalue 0.75) 4.0)))
      (elif (> _returnvalue 0.25)
        (return (`KismetMathLibrary.LinearColorLerp` (struct :`B` 1.0 :`A` 1.0) (struct :`G` 1.0 :`A` 1.0) (* (- _returnvalue 0.75) 4.0)))
        (else
          (return (`KismetMathLibrary.LinearColorLerp` (struct :`R` 1.0 :`G` 1.0 :`B` 1.0 :`A` 1.0) (struct :`B` 1.0 :`A` 1.0) (* _returnvalue 4.0))))))))

(fn `UserConstructionScript`
  (set `self.LastPosition` (`self.K2_GetActorLocation`)))