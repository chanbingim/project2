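; BP_Grenade_Test is a test grenade actor that explodes three seconds after it begins play.
; Detonation spawns an explosion emitter and sound, fires a radial force impulse, and asks BP_TPSGameState to spawn a debug-drawn area-of-effect check.
; The AOE reports each hit actor through a delegate that only prints its name.
; The mesh is then hidden and the actor destroys itself after a short delay.
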(event `self.ReceiveBeginPlay`
  (`KismetSystemLibrary.Delay` 3.0)
  (`self.OnDetonated`))

(event `OnDetonated`
  (bind _returnvalue (`self.K2_GetActorLocation`))
  (`GameplayStatics.SpawnEmitterAtLocation` "/Game/StarterContent/Particles/P_Explosion.P_Explosion" (`self.K2_GetActorLocation`))
  (`RadialForceComponent.FireImpulse` (`self.RadialForce`))
  (`GameplayStatics.PlaySoundAtLocation` "/Game/StarterContent/Audio/Explosion_Cue.Explosion_Cue" _returnvalue (struct) 1.0 1.0 0.0 null null null null)
  (bind _asbp_tpsgame_state (cast `/Game/Default/AOESystem/BP_TPSGameState` (`GameplayStatics.GetGameState`)))
  (`/Game/Default/AOESystem/BP_TPSGameState.SpawnAOE` _asbp_tpsgame_state _returnvalue 300.0 false self (delegate `Event`) 1.0 (struct :`R` 1.0 :`B` 0.013355 :`A` 1.0))
  (`SceneComponent.SetHiddenInGame` (`self.StaticMesh`) true false)
  (`KismetSystemLibrary.Delay` 3.0)
  (`self.K2_DestroyActor`))

(event `Event`
  (params (`Hit Actor` :type "Actor Object Reference"))
  (`KismetSystemLibrary.PrintString` (`KismetSystemLibrary.GetDisplayName` `Hit Actor`)))

(fn `UserConstructionScript`)