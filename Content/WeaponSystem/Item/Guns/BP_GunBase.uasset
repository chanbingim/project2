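; BP_GunBase is the base gun actor: players pick it up, it toggles between equipped and physics-dropped states, and it handles ammo, fire feedback and magazine spawning.
; An enum-indexed attachment array spawns parts onto sockets; optics set ADS camera offset and FOV, suppressors override muzzle, sound and noise radius.
; A timeline drives controller recoil, reversing on stop with recovery scaled by pitch drift.
; The laser sight uses a traced beam emitter.
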(event `self.ReceiveBeginPlay`
  (`parent.ReceiveBeginPlay`)
  (`self.Update Camera Fov`)
  (`KismetArrayLibrary.Array_Resize` (`self.Attachments`) (enumcount `/Game/WeaponSystem/GunSmithSystem/Enum/E_AttachmentTypes`)))

(event `Play Gun Fire Animation and FX`
  (bind _skeletalmesh (`self.SkeletalMesh`))
  (`|PlayMontage` _skeletalmesh (`self.GunFireAnim`)
    (:`then`
      (`GameplayStatics.SpawnSoundAttached` (`self.GunFireSound`) _skeletalmesh "None" (0.0 0.0 0.0) (struct) "KeepRelativeOffset" false 1.0 1.0 0.0 null null))))

(event `/Game/WeaponSystem/Interaction/InteractionInterface.On Interacted`
  (params (Player :type "/Game/WeaponSystem/Player/BP_Player2 Object Reference"))
  (`self.AttachGun` Player))

(event `/Game/WeaponSystem/Interaction/InteractionInterface.On Interacted Enemy`
  (params (Enemy :type "/Game/AI/BP_MyCharacterAI Object Reference"))
  (`self.AttachGun_Enemy` Enemy))

(event `SpawnMagazine`
  (bind _returnvalue (`SceneComponent.GetSocketLocation` (`self.SkeletalMesh`) "Magazine"))
  (bind (_returnvalue_location _returnvalue_rotation) (`KismetMathLibrary.BreakTransform` (`SceneComponent.GetSocketTransform` (`self.SkeletalMesh`) "None" "RTS_World")))
  (`self.MagazineObj`
    (:`then`
      (bind _output_get (set `self.Magazine Velocity` _returnvalue))
      (`KismetSystemLibrary.Delay` (* (`GameplayStatics.GetWorldDeltaSeconds`) 5.0))
      (set `self.Magazine Velocity` (- _returnvalue _output_get))
      (`|SpawnActorFromClass` (`self.MagazineObj`) (`KismetMathLibrary.MakeTransform` _returnvalue_location _returnvalue_rotation) "AlwaysSpawn" "OverrideRootScale" (`self.GetOwner`) null))
    (:`else`)))

(event `/Game/WeaponSystem/GunSmithSystem/BPI_Attachments.AddAttachment`
  (params (`Attachments to add` :type "/Game/WeaponSystem/GunSmithSystem/Enum/E_AttachmentTypes Enum" :default "NewEnumerator0"))
  (`/Game/WeaponSystem/GunSmithSystem/BPI_Attachments.RemoveAttachment` `Attachments to add`)
  (bind _returnvalue (`|SpawnActorFromClass` (select `/Game/WeaponSystem/GunSmithSystem/Enum/E_AttachmentTypes` `Attachments to add` :`NewEnumerator0` "/Game/WeaponSystem/Item/Attachments/BP_OpticsBase.BP_OpticsBase_C" :`NewEnumerator3` "/Game/WeaponSystem/Item/Attachments/BP_SupressorBase.BP_SupressorBase_C" :`NewEnumerator7` "/Game/WeaponSystem/Item/Attachments/BP_LaserSightBase.BP_LaserSightBase_C" :!type "Actor Class Reference") (`KismetMathLibrary.MakeTransform` (0.0 0.0 0.0)) "Undefined" "OverrideRootScale" null null))
  (`self.K2_AttachToComponent` _returnvalue (`self.SkeletalMesh`) (select `/Game/WeaponSystem/GunSmithSystem/Enum/E_AttachmentTypes` `Attachments to add` :`NewEnumerator0` "AttachmentSocketScope" :`NewEnumerator1` "Magazine" :`NewEnumerator2` "AttachmentSocketBarrelLowFront" :`NewEnumerator3` "AttachmentSocketSilencer" :`NewEnumerator6` "AttachmentSocketBarrelLeft" :`NewEnumerator7` "LaserSightSocket" :!type "Name") "KeepRelative" "KeepRelative" "KeepRelative" true)
  (`KismetArrayLibrary.Array_Set` (`self.Attachments`) (`KismetMathLibrary.Conv_ByteToInt` `Attachments to add`) _returnvalue)
  (`self.Update Camera Fov`)
  (`self.SetLaserSight`))

(event `/Game/WeaponSystem/GunSmithSystem/BPI_Attachments.RemoveAttachment`
  (params (`Attachment to Remove` :type "/Game/WeaponSystem/GunSmithSystem/Enum/E_AttachmentTypes Enum" :default "NewEnumerator0"))
  (bind _output (`|GetArrayItem` (`self.Attachments`) (`KismetMathLibrary.Conv_ByteToInt` `Attachment to Remove`)))
  (`/Engine/EditorBlueprintResources/StandardMacros.IsValid` _output
    (:`Is Valid`
      (`self.K2_DestroyActor` _output))))

(event `LaserSight On/Off`
  (params (Off :type Boolean))
  (set `self.EnableLaserSight` Off)
  (`/Engine/EditorBlueprintResources/StandardMacros.IsValid` (`self.LaserSightComponent`)
    (:`Is Valid`
      (`SceneComponent.SetVisibility` (`self.LaserSightComponent`) (`self.EnableLaserSight`) false))))

(event `OnFire`
  (bind _recoilrate (`self.RecoilRate`))
  (bind _returnvalue (`KismetMathLibrary.MapRangeClamped` (`KismetMathLibrary.Abs` (.pitch (`KismetMathLibrary.NormalizedDeltaRotator` (`self.OriginRotation`) (`self.PostRecoilRotation`)))) 0.0 (`self.RecoilMaxThreshold`) 0.0 1.0))
  (`TimelineComponent.SetPlayRate` (`self.RecoilTimeline`) 1.0)
  (`|ExecutionSequence`
    (:`then_0`
      (`/Engine/EditorBlueprintResources/StandardMacros.DoOnce` false :!label _label
        (:`Completed`
          (set `self.OriginRotation` (`Controller.GetControlRotation` (`GameplayStatics.GetPlayerController` 0))))))
    (:`then_1`
      (bind (_direction _pitchinput _yawinput) (`Timeline|RecoilTimeline` :!label _label_2)
        (:`Update`
          (switch `ETimelineDirection` _direction
            (:`Forward`
              (`self.AddControllerPitchAndYaw` _pitchinput _yawinput))
            (:`Backward`
              (`|ExecutionSequence`
                (:`then_0`
                  (`/Engine/EditorBlueprintResources/StandardMacros.DoOnce` false :!label _label_3
                    (:`Completed`
                      (set `self.PostRecoilRotation` (`Controller.GetControlRotation` (`GameplayStatics.GetPlayerController` 0))))))
                (:`then_1`
                  (`self.AddControllerPitchAndYaw` (* (* _pitchinput -1.0) _recoilrate _returnvalue) (* (* _yawinput -1.0) _recoilrate _returnvalue)))))))
        (:`Finished`
          (switch `ETimelineDirection` _direction
            (:`Backward`
              (`self.ResetRecoil`))))))))

(event `StopFire`
  (`TimelineComponent.SetPlayRate` (`self.RecoilTimeline`) (`self.RecoilRate`))
  (goto _label_2 :!via `Reverse`))

(event `ResetRecoil`
  (`|ExecutionSequence`
    (:`then_0`
      (goto _label :!via `Reset`))
    (:`then_1`
      (goto _label_3 :!via `Reset`))))

(fn `AddControllerPitchAndYaw`
  (params (Pitch :type "Float (single-precision)") (Yaw :type "Float (single-precision)"))
  (bind _returnvalue (`GameplayStatics.GetPlayerController` 0))
  (`PlayerController.AddPitchInput` _returnvalue Pitch)
  (`PlayerController.AddYawInput` _returnvalue Yaw))

(fn `ChangeState`
  (params (NewState :type "/Game/WeaponSystem/Item/Guns/E_GunState Enum" :default "NewEnumerator0"))
  (bind _skeletalmesh (`self.SkeletalMesh`))
  (bind _skeletalmesh_2 (`self.SkeletalMesh`))
  (bind _output_get (set `self.GunState` NewState))
  (switch `/Game/WeaponSystem/Item/Guns/E_GunState` _output_get
    (:`NewEnumerator0`
      (`PrimitiveComponent.SetCollisionProfileName` (`self.Sphere`) "OverlapAllDynamic" true)
      (`PrimitiveComponent.SetSimulatePhysics` _skeletalmesh true)
      (`PrimitiveComponent.SetCollisionProfileName` _skeletalmesh "DroppedGun" true))
    (:`NewEnumerator1`
      (`PrimitiveComponent.SetCollisionProfileName` (`self.Sphere`) "NoCollision" false)
      (`PrimitiveComponent.SetSimulatePhysics` _skeletalmesh_2 false)
      (`PrimitiveComponent.SetCollisionProfileName` _skeletalmesh_2 "NoCollision" false)
      (`SceneComponent.ResetRelativeTransform` (`self.SkeletalMesh`)))))

(fn `Decrease Ammo`
  (set `self.CurrClip` (`KismetMathLibrary.Clamp` (- (`self.CurrClip`) 1) 0 (`self.MaxClip`))))

(fn `DropGun`
  (`self.ChangeState` "NewEnumerator0")
  (`self.SetOwner` null))

(fn `GetAdsCameraOffset`
  (returns (Offset :type "Vector Structure"))
  (bind _output (`|GetArrayItem` (`self.Attachments`) (`KismetMathLibrary.Conv_ByteToInt` (enumliteral `/Game/WeaponSystem/GunSmithSystem/Enum/E_AttachmentTypes` "NewEnumerator0"))))
  (`/Engine/EditorBlueprintResources/StandardMacros.IsValid` _output
    (:`Is Valid`
      (bind _asbp_optics_base (cast `/Game/WeaponSystem/Item/Attachments/BP_OpticsBase` _output)
        (:`then`
          (return (`/Game/WeaponSystem/Item/Attachments/BP_OpticsBase.CameraOffset` _asbp_optics_base)))
        (:`CastFailed`
          _)))
    (:`Is Not Valid`
      _))
  (return (0.0 0.0 0.0)))

(fn `GetFireSound`
  (returns (FireSound :type "SoundBase Object Reference"))
  (bind (_output _valid) (`self.IsAttachmentExist` "NewEnumerator3"))
  (if _valid
    (bind _asbp_supressor_base (cast `/Game/WeaponSystem/Item/Attachments/BP_SupressorBase` _output))
    (return (`/Game/WeaponSystem/Item/Attachments/BP_SupressorBase.SupressorFireSound` _asbp_supressor_base))
    (else
      (return (`self.GunFireSound`)))))

(fn `GetMuzzlePosition`
  (returns (`Muzzle Location` :type "Vector Structure") (`Muzzle Rotation` :type "Rotator Structure"))
  (bind _skeletalmesh (`self.SkeletalMesh`))
  (bind _skeletalmesh_2 (`self.SkeletalMesh`))
  (bind _muzzleflash (`self.MuzzleFlash`))
  (bind _asbp_supressor_base (cast `/Game/WeaponSystem/Item/Attachments/BP_SupressorBase` (`|GetArrayItem` (`self.Attachments`) (`KismetMathLibrary.Conv_ByteToInt` (enumliteral `/Game/WeaponSystem/GunSmithSystem/Enum/E_AttachmentTypes` "NewEnumerator3"))))
    (:`then`
      (bind _supressormuzzleflash (`/Game/WeaponSystem/Item/Attachments/BP_SupressorBase.SupressorMuzzleFlash` _asbp_supressor_base))
      (return (`SceneComponent.GetSocketLocation` _skeletalmesh _supressormuzzleflash) (`SceneComponent.GetSocketRotation` _skeletalmesh _supressormuzzleflash)))
    (:`CastFailed`
      (return (`SceneComponent.GetSocketLocation` _skeletalmesh_2 _muzzleflash) (`SceneComponent.GetSocketRotation` _skeletalmesh_2 _muzzleflash)))))

(fn `GetSoundRadius`
  (returns (SoundRadius :type "Float (double-precision)"))
  (bind (_output _valid) (`self.IsAttachmentExist` "NewEnumerator3"))
  (if _valid
    (bind _asbp_supressor_base (cast `/Game/WeaponSystem/Item/Attachments/BP_SupressorBase` _output))
    (return (`/Game/WeaponSystem/Item/Attachments/BP_SupressorBase.SoundRadius` _asbp_supressor_base))
    (else
      (return (`self.SoundRadius`)))))

(fn `IsAttachmentExist`
  (params (Attachment :type "/Game/WeaponSystem/GunSmithSystem/Enum/E_AttachmentTypes Enum" :default "NewEnumerator0"))
  (returns (Output :type "Actor Object Reference") (valid :type Boolean))
  (bind _output (`|GetArrayItem` (`self.Attachments`) (`KismetMathLibrary.Conv_ByteToInt` Attachment)))
  (`/Engine/EditorBlueprintResources/StandardMacros.IsValid` _output
    (:`Is Valid`
      (return _output true))
    (:`Is Not Valid`
      (return null false))))

(fn `Set Magazine Visual`
  (params (ToHide :type Boolean))
  (if ToHide
    (`SkinnedMeshComponent.HideBoneByName` (`self.SkeletalMesh`) "Magazin" "PBO_None")
    (else
      (`SkinnedMeshComponent.UnHideBoneByName` (`self.SkeletalMesh`) "Magazin"))))

(fn `SetLaserSight`
  (locals (LaserSight :type "/Game/WeaponSystem/Item/Attachments/BP_LaserSightBase Object Reference") (AdsCamera :type "/Game/WeaponSystem/Component/ADS_Camera Object Reference"))
  (bind (_output _valid) (`self.IsAttachmentExist` "NewEnumerator7"))
  (if _valid
    (bind _asbp_laser_sight_base (cast `/Game/WeaponSystem/Item/Attachments/BP_LaserSightBase` _output))
    (if (`self.EnableLaserSight`)
      (bind _returnvalue (`GameplayStatics.SpawnEmitterAttached` (`self.Weapon LaserSight FX`) (`/Game/WeaponSystem/Item/Attachments/BP_AttachmentBase.StaticMesh` _asbp_laser_sight_base) (`/Game/WeaponSystem/Item/Attachments/BP_LaserSightBase.LaserStart` _asbp_laser_sight_base)))
      (set `self.LaserSightComponent` _returnvalue))))

(fn `Update Ads Camera Position`
  (bind _asads_camera (cast `/Game/WeaponSystem/Component/ADS_Camera` (`ChildActorComponent.ChildActor` (`self.ADS Camera System`))))
  (`SceneComponent.K2_AttachToComponent` (`/Game/WeaponSystem/Component/ADS_Camera.SpringArm` _asads_camera) (`self.SkeletalMesh`) "AimingCameraLocation" "KeepRelative" "KeepRelative" "KeepRelative" true))

(fn `Update Attachments`
  (`self.Update Camera Fov`))

(fn `Update Camera Fov`
  (bind _asads_camera (cast `/Game/WeaponSystem/Component/ADS_Camera` (`ChildActorComponent.ChildActor` (`self.ADS Camera System`)))
    (:`then`
      (bind _asbp_optics_base (cast `/Game/WeaponSystem/Item/Attachments/BP_OpticsBase` (`|GetArrayItem` (`self.Attachments`) (`KismetMathLibrary.Conv_ByteToInt` (enumliteral `/Game/WeaponSystem/GunSmithSystem/Enum/E_AttachmentTypes` "NewEnumerator0"))))
        (:`then`
          (`/Game/WeaponSystem/Component/ADS_Camera.CameraFovSetting` _asads_camera (`/Game/WeaponSystem/Item/Attachments/BP_OpticsBase.CameraFOV` _asbp_optics_base)))
        (:`CastFailed`
          (`/Game/WeaponSystem/Component/ADS_Camera.CameraFovSetting` _asads_camera (`self.DefaultCameraFov`) :!label _label))))
    (:`CastFailed`
      (goto _label))))

(fn `UpdateLaserSight`
  (params (Hit :type Boolean) (Location :type "Vector Structure"))
  (locals (LaserSight :type "/Game/WeaponSystem/Item/Attachments/BP_LaserSightBase Object Reference") (AdsCamera :type "/Game/WeaponSystem/Component/ADS_Camera Object Reference") (`Hit Var` :type Boolean) (`Location Var` :type "Vector Structure"))
  (bind _lasersightcomponent (`self.LaserSightComponent`))
  (bind _lasersight (`local.LaserSight`))
  (bind _laserlocation (`/Game/WeaponSystem/Item/Attachments/BP_LaserSightBase.GetLaserStartSocket` _lasersight))
  (set `local.Location Var` Location)
  (set `local.Hit Var` Hit)
  (bind (_output _valid) (`self.IsAttachmentExist` "NewEnumerator7"))
  (if _valid
    (bind _asbp_laser_sight_base (cast `/Game/WeaponSystem/Item/Attachments/BP_LaserSightBase` _output))
    (set `local.LaserSight` _asbp_laser_sight_base)
    (bind _asads_camera (cast `/Game/WeaponSystem/Component/ADS_Camera` (`ChildActorComponent.ChildActor` (`self.ADS Camera System`))))
    (set `local.AdsCamera` _asads_camera)
    (`/Engine/EditorBlueprintResources/StandardMacros.IsValid` _lasersightcomponent
      (:`Is Valid`
        (if (`self.EnableLaserSight`)
          (`ParticleSystemComponent.SetBeamSourcePoint` _lasersightcomponent 0 _laserlocation 0)
          (bind _outhit (`KismetSystemLibrary.LineTraceSingle` _laserlocation (+ _laserlocation (* (`SceneComponent.GetForwardVector` (`/Game/WeaponSystem/Item/Attachments/BP_LaserSightBase.Arrow` _lasersight)) 10000.0)) "TraceTypeQuery1"))
          (`ParticleSystemComponent.SetBeamTargetPoint` (`self.LaserSightComponent`) 0 (select `bool` (`local.Hit Var`) :`false` (`.TraceEnd` (`GameplayStatics.BreakHitResult` _outhit)) :`true` (`local.Location Var`)) 0))))))

(fn `UserConstructionScript`
  (`parent.UserConstructionScript`))