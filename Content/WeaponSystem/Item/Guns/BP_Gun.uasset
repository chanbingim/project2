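; Interactable gun actor that BP_Player2 picks up, fires and drops, switching collision and mesh physics between Dropped and Equipped states.
; Fire dispatches on single, burst or full-auto mode, with burst and full-auto looping through delayed recursive events, and reloads from the player's ammo when unable to shoot.
; SpawnBullet launches a projectile from the muzzle socket toward the camera's aim point, adds a muzzle flash and decrements ammo.
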(event `self.ReceiveBeginPlay`
  (`self.Set GunState` "NewEnumerator0"))

(event `/Game/WeaponSystem/Interaction/InteractionInterface.On Interacted`
  (params (Player :type "/Game/WeaponSystem/Player/BP_Player2 Object Reference"))
  (`/Game/WeaponSystem/Player/BP_Player2.PickUp Gun` Player self)
  (`self.Set GunState` self "NewEnumerator1")
  (if (`/Game/WeaponSystem/Player/BP_Player2.GrenadeMode` Player)
    (`self.SetActorHiddenInGame` true)))

(event `Check Can Shoot`
  ;[1 1 1] 총알 체크
  (if (> (`self.Ammo`) 0)
    (set `self.canShoot` true)
    (else
      (set `self.canShoot` false))))

(event `Full auto Fire`
  (params (AimCamera :type "CameraComponent Object Reference"))
  (if (`self.canShoot`)
    (if (`self.canShoot`)
      (`KismetSystemLibrary.Delay` 0.15)
      (`self.SpawnBullet` AimCamera)
      (switch `/Game/WeaponSystem/Item/Guns/E_SelectorType` (`self.SelectType`)
        (:`NewEnumerator2`
          (if (`self.IsShooting`)
            (`self.Full auto Fire` AimCamera)))))
    (else
      (set `self.IsShooting` false))))

(event `Burst Fire`
  (params (AimCamera :type "CameraComponent Object Reference"))
  (set `self.IsBurstShot` true)
  (if (!= (`self.N`) 3)
    (if (`self.canShoot`)
      (`KismetSystemLibrary.Delay` 0.05)
      (`self.SpawnBullet` AimCamera)
      (set `self.N` (+ (`self.N`) 1))
      (`self.Burst Fire` AimCamera)
      (else
        (set `self.N` 0 :!label _label)
        (set `self.IsBurstShot` false)))
    (else
      (goto _label))))

(event `Reload Gun`
  (bind _asbp_player_2 (cast `/Game/WeaponSystem/Player/BP_Player2` (`self.GetOwner`)))
  (if (== (`self.MaxAmmo`) (`self.Ammo`))
    (`KismetSystemLibrary.PrintString` "Full Ammo")
    (else
      (bind _ammo (`/Game/WeaponSystem/Player/BP_Player2.Ammo` _asbp_player_2))
      (if (> _ammo 0)
        (if (> _ammo (`self.MaxAmmo`))
          (bind _output_get (set `/Game/WeaponSystem/Player/BP_Player2.Ammo` (- _ammo (- (`self.MaxAmmo`) (`self.Ammo`))) _asbp_player_2))
          (set `self.Ammo` (`self.MaxAmmo`))
          (`KismetSystemLibrary.PrintString` (`KismetStringLibrary.Concat_StrStr` (`KismetStringLibrary.Conv_IntToString` _output_get) "Rounds Left"))
          (else
            (set `self.Ammo` _ammo)
            (set `/Game/WeaponSystem/Player/BP_Player2.Ammo` 0 _asbp_player_2)))
        (`self.Check Can Shoot`)
        (`KismetSystemLibrary.PrintString` "Reload Complete!")
        (else
          (`KismetSystemLibrary.PrintString` "Reload Failed"))))))

(fn `DropGun`
  (`self.Set GunState` "NewEnumerator0")
  (`self.SetOwner` null))

(fn `Fire`
  (params (AimCamera :type "CameraComponent Object Reference"))
  (`self.Check Can Shoot`)
  (if (`self.canShoot`)
    (set `self.IsShooting` true)
    (switch `/Game/WeaponSystem/Item/Guns/E_SelectorType` (`self.SelectType`)
      (:`NewEnumerator0`
        (`self.SpawnBullet` AimCamera))
      (:`NewEnumerator1`
        (if (not (`self.IsBurstShot`))
          (`self.Burst Fire` AimCamera)))
      (:`NewEnumerator2`
        (`self.Full auto Fire` AimCamera)))
    (else
      (`self.Reload Gun`))))

(fn `Get Interaction Text`
  (returns (Text :type Text))
  (return (`parent.Get Interaction Text`)))

(fn `Get Interaction TextAttach`
  (returns (AttachComponent :type "SceneComponent Object Reference"))
  (return null))

(fn `Release Fire`
  (set `self.IsShooting` false))

(fn `Set GunState`
  (params (`New Gun State` :type "/Game/WeaponSystem/Item/Guns/E_GunState Enum" :default "NewEnumerator0"))
  (bind _skeletalmesh (`self.SkeletalMesh`))
  (bind _skeletalmesh_2 (`self.SkeletalMesh`))
  (bind _output_get (set `self.GunState` `New Gun State`))
  (switch `/Game/WeaponSystem/Item/Guns/E_GunState` _output_get
    (:`NewEnumerator0`
      (`PrimitiveComponent.SetCollisionProfileName` (`self.Sphere`) "OverlapAllDynamic" true)
      (`PrimitiveComponent.SetSimulatePhysics` _skeletalmesh true)
      (`PrimitiveComponent.SetCollisionProfileName` _skeletalmesh "DroppedGun" true))
    (:`NewEnumerator1`
      (`PrimitiveComponent.SetCollisionProfileName` (`self.Sphere`) "NoCollision" false)
      (`PrimitiveComponent.SetSimulatePhysics` _skeletalmesh_2 false)
      (`PrimitiveComponent.SetCollisionProfileName` _skeletalmesh_2 "NoCollision" false)
      (`SceneComponent.ResetRelativeTransform` (`self.SkeletalMesh`)))))

(fn `SpawnBullet`
  (params (AimCamera :type "CameraComponent Object Reference"))
  (bind _returnvalue (`SceneComponent.GetSocketLocation` (`self.SkeletalMesh`) "b_gun_muzzleflash"))
  (if (`self.canShoot`)
    (`|SpawnActorFromClass` (`self.Bullet`) (`KismetMathLibrary.MakeTransform` _returnvalue) "Undefined" "OverrideRootScale" self (* (`KismetMathLibrary.Normal` (- (+ (`SceneComponent.K2_GetComponentLocation` AimCamera) (* (`SceneComponent.GetForwardVector` AimCamera) (`self.MaxDistance`))) _returnvalue)) (`self.BulletSpeed`)) null)
    (`|SpawnActorFromClass` "/Game/WeaponSystem/Item/Bullets/BP_MuzzleFlash.BP_MuzzleFlash_C" (`KismetMathLibrary.MakeTransform` _returnvalue) "Undefined" "OverrideRootScale" null null)
    (bind _output_get (set `self.Ammo` (- (`self.Ammo`) 1)))
    (`self.Check Can Shoot`)
    (`KismetSystemLibrary.PrintString` (`KismetStringLibrary.Concat_StrStr` (`KismetStringLibrary.Conv_IntToString` _output_get) "/" (`KismetStringLibrary.Conv_IntToString` (`self.MaxAmmo`))))))

(fn `Switch Selector`
  (switch `/Game/WeaponSystem/Item/Guns/E_SelectorType` (`self.SelectType`)
    (:`NewEnumerator0`
      (bind _output_get (set `self.SelectType` "NewEnumerator1"))
      (`KismetSystemLibrary.PrintString` (`|GetEnumeratorNameAsString` _output_get)))
    (:`NewEnumerator1`
      (bind _output_get_2 (set `self.SelectType` "NewEnumerator2"))
      (`KismetSystemLibrary.PrintString` (`|GetEnumeratorNameAsString` _output_get_2)))
    (:`NewEnumerator2`
      (bind _output_get_3 (set `self.SelectType` "NewEnumerator0"))
      (`KismetSystemLibrary.PrintString` (`|GetEnumeratorNameAsString` _output_get_3)))))

(fn `UserConstructionScript`
  (`parent.UserConstructionScript`))