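; BP_RifleTest2 is a test rifle Blueprint in the weapon system that adds an adjustable sniper zoom to its aim-down-sights camera.
; The SniperZoom event adds the incoming value to a clamped FOV, then passes it to the ADS_Camera child actor through CameraFovSetting.
; BeginPlay, overlap and Tick are disabled placeholders, and the construction script only calls its parent.
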(event `Sniper Zoom`
  (params (Value :type "Float (double-precision)"))
  (bind _output_get (set `self.Fov` (`KismetMathLibrary.FClamp` (+ (`self.Fov`) Value) 10.0 60.0)))
  (bind _asads_camera (cast `/Game/WeaponSystem/Component/ADS_Camera` (`ChildActorComponent.ChildActor` (`self.ADS Camera System`))))
  (`/Game/WeaponSystem/Component/ADS_Camera.CameraFovSetting` _asads_camera _output_get))

(fn `UserConstructionScript`
  (`parent.UserConstructionScript`))