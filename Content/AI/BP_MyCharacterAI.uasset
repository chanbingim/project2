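; AI character Blueprint that previews its sensing ranges and plays an assassination (Amsal) death reaction.
; The construction script flushes persistent debug lines, then draws nested sight cones, a hearing circle and an active-range sphere from its sense variables.
; PlayAmsalMontage disables movement, sets the mesh constraint mode and plays the death montage behind a DoOnce that resets on completion.
; SpawnGun1 spawns and returns an actor of any valid class passed in.
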(event `self.ReceiveBeginPlay`)

(event `self.PlayAmsalMontage`
  (`CharacterMovementComponent.DisableMovement` (`self.CharacterMovement`))
  (`/Engine/EditorBlueprintResources/StandardMacros.DoOnce` false :!label _label
    (:`Completed`
      (`PrimitiveComponent.SetConstraintMode` (`self.Mesh`) (`self.Constraint Mode`))
      (`|PlayMontage` (`self.Mesh`) "/Game/AI/Animation/Retarget/RE_Ai_Amsal_Death.RE_Ai_Amsal_Death"
        (:`OnCompleted`
          (goto _label :!via `Reset`))))))

(fn `SpawnGun1`
  (params (Class :type "/Game/WeaponSystem/Item/Guns/BP_GunBase Class Reference"))
  (returns (`AsBP Gun Base` :type "/Game/WeaponSystem/Item/Guns/BP_GunBase Object Reference"))
  (if (`KismetSystemLibrary.IsValidClass` Class)
    (bind _returnvalue (`|SpawnActorFromClass` Class (`KismetMathLibrary.MakeTransform` (0.0 0.0 0.0)) "Undefined" "OverrideRootScale" null null))
    (return _returnvalue)))

(fn `UserConstructionScript`
  (locals (Duration :type "Float (double-precision)" :default 2.0) (Thick :type "Float (double-precision)" :default 2.0))
  (bind _sense_sight_degrees (`self.Sense_Sight_Degrees`))
  (`KismetSystemLibrary.FlushPersistentDebugLines`)
  (`|ExecutionSequence`
    (:`then_0`
      (for _index (range (+ (`KismetMathLibrary.FTrunc` (/ _sense_sight_degrees 20.0)) 1))
        (bind _returnvalue (- _sense_sight_degrees (* _index 20)))
        (`KismetSystemLibrary.DrawDebugConeInDegrees` (`self.K2_GetActorLocation`) (`self.GetActorForwardVector`) (`self.Sense_Sight_Range`) _returnvalue _returnvalue 12 (struct :`G` 1.0 :`A` 1.0) (`local.Duration`) (`local.Thick`))))
    (:`then_1`
      (`KismetSystemLibrary.DrawDebugCircle` (`self.K2_GetActorLocation`) (`self.Sense_Hearing_Range`) 30 (struct :`R` 1.0 :`G` 1.0 :`A` 1.0) (`local.Duration`) (`local.Thick`) (0.0 1.0 0.0) (1.0 0.0 0.0)))
    (:`then_2`
      (`KismetSystemLibrary.DrawDebugSphere` (`self.K2_GetActorLocation`) (`self.Active_Range`) 20 (struct :`A` 1.0) (`local.Duration`) (`local.Thick`)))))