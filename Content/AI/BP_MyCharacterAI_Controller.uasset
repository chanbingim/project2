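; AI controller that drives an on-screen detection meter (WD_Meter) for its controlled pawn.
; WidgetCall creates the meter, and UpdatePercent maps SenseCurrent against the pawn's SenseSearchMax to a flipbook frame.
; Tick points the meter toward the pawn relative to player view and scales it by 2D distance.
; The meter is removed on request, on death, or shortly after a toggle when blackboard state reaches 4.
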(event `self.Widget_Call`
  (bind _returnvalue (`|CreateWidget` "/Game/WeaponSystem/WIdget/WD_Meter.WD_Meter_C"))
  (bind _output_get (set `self.WD_Meter` _returnvalue))
  (`UserWidget.AddToViewport` _output_get 0)
  (set `self.SetViewPort` true))

(event `UpdatePercent`
  (bind _wd_meter (`self.WD_Meter`))
  (if (`self.SetViewPort`)
    (`PaperFlipbookUserWidget.SetPlaybackPositionInFrames` (`/Game/WeaponSystem/WIdget/WD_Meter.WDMeter` _wd_meter) (`KismetMathLibrary.FTrunc` (* (`PaperFlipbookUserWidget.GetFlipbookLengthInFrames` (`/Game/WeaponSystem/WIdget/WD_Meter.WDMeter` (`self.WD_Meter`))) (/ (`self.Sense_Current`) (`MyCharacterAI.Sense_Search_Max` (`self.OwnerPawn`))))))
    (if (== (`BlackboardComponent.GetValueAsEnum` (`AIBlueprintHelperLibrary.GetBlackboard` null) (`self.E_CurrentState`)) 4)
      (`/Game/WeaponSystem/WIdget/WD_Meter.ToggleEvent` _wd_meter)
      (`KismetSystemLibrary.Delay` 0.3)
      (bind _wd_meter_2 (`self.WD_Meter` :!label _label)
        (:`then`
          (`Widget.RemoveFromParent` _wd_meter_2)
          (set `self.SetViewPort` false))
        (:`else`)))))

(event `self.ReMoveWidget`
  (goto _label))

(event `self.ReceiveTick`
  (params (DeltaSeconds :type "Float (single-precision)"))
  (bind _returnvalue (`self.K2_GetActorLocation` (`self.K2_GetPawn`)))
  (bind _returnvalue_2 (`self.K2_GetActorLocation` (`GameplayStatics.GetPlayerCharacter` 0)))
  (bind (_returnvalue_roll _returnvalue_pitch _returnvalue_yaw) (`KismetMathLibrary.BreakRotator` (`KismetMathLibrary.NormalizedDeltaRotator` (`KismetMathLibrary.FindLookAtRotation` _returnvalue_2 _returnvalue) (`self.GetControlRotation` (`GameplayStatics.GetPlayerController` 0)))))
  (bind _returnvalue_3 (`KismetMathLibrary.FClamp` (/ (`KismetMathLibrary.Vector_Distance2D` _returnvalue _returnvalue_2) 1000.0) 0.5))
  (bind _wd_meter (`self.WD_Meter`)
    (:`then`
      (`|ExecutionSequence`
        (:`then_0`
          (`/Game/WeaponSystem/WIdget/WD_Meter.UpdateAngle` _wd_meter _returnvalue_yaw))
        (:`then_1`
          (`/Engine/EditorBlueprintResources/StandardMacros.CompareFloat` _returnvalue_3 0.5
            (:`>`
              (bind _output_get (set `self.Distance` (- 1.5 _returnvalue_3)))
              (set `self.Scale` (`KismetMathLibrary.MakeVector2D` _output_get _output_get)))
            (:`<`
              (bind _output_get_2 (set `self.Distance` _returnvalue_3))
              (set `self.Scale` (`KismetMathLibrary.MakeVector2D` _output_get_2 _output_get_2))))
          (`/Game/WeaponSystem/WIdget/WD_Meter.UpdateSize` _wd_meter (`self.Scale`))))
      (`self.UpdatePercent`)
      (if (`|EnumEquality` (`self.Current_State`) "E_StateDead")
        (`Widget.RemoveFromParent` (`self.WD_Meter`))))
    (:`else`)))

(fn `UserConstructionScript`)