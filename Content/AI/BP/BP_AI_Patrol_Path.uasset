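; AI patrol path actor that defines a route as a spline and labels its points for level designers.
; The construction script loops over every spline point and calls ShowSplineIndex, which adds a text render component above that point showing its index number.
; The event graph holds no runtime logic.
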(event `self.ReceiveTick`
  (params (DeltaSeconds :type "Float (single-precision)")))

(fn `ShowSplineIndex`
  (params (Index :type Integer))
  (bind _returnvalue (`AddComponent|NODE_AddTextRenderComponent-0` :`RelativeTransform` (`KismetMathLibrary.MakeTransform` (+ (`SplineComponent.GetLocationAtSplinePoint` (`self.Spline`) (`local.Index`) "Local") (0.0 0.0 200.0)))))
  (`TextRenderComponent.K2_SetText` _returnvalue (`KismetTextLibrary.Conv_IntToText` (`local.Index`)))
  (return))

(fn `UserConstructionScript`
  (for _index (range (`SplineComponent.GetNumberOfSplinePoints` (`self.Spline`)))
    (`self.ShowSplineIndex` _index)))