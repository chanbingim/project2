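; BP_AOECharacter is a character with clamped health that can fire a damaging area-of-effect around itself on input.
; On BeginPlay it fills health and passes itself to the health widget as an interface, exposing the health ratio.
; The Spawn AOE input asks BP_TPSGameState for a line-of-sight AOE with debug drawing, supplying a delegate that sends a damage interface message to each actor hit.
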(event `self.ReceiveBeginPlay`
  (`parent.ReceiveBeginPlay`)
  (set `self.Health` (`self.MaxHealth`))
  (bind _asuwb_health (cast `/Game/Default/AOESystem/UWB_Health` (`WidgetComponent.GetUserWidgetObject` (`self.HealthWidget`))))
  (set `/Game/Default/AOESystem/UWB_Health.HealthInterface` self _asuwb_health))

(event `/Game/Default/AOESystem/BPI_HealthInterface.Heal`
  (params (Amount :type "Float (double-precision)"))
  (set `self.Health` (`KismetMathLibrary.FClamp` (+ (`self.Health`) Amount) 0.0 (`self.MaxHealth`))))

(event `/Game/Default/AOESystem/BPI_HealthInterface.Damage`
  (params (Amount :type "Float (double-precision)"))
  (set `self.Health` (`KismetMathLibrary.FClamp` (- (`self.Health`) Amount) 0.0 (`self.MaxHealth`))))

(event `InputAction|Spawn AOE`
  (params (Key :type "Key Structure"))
  (:`Pressed`
    (bind _asbp_tpsgame_state (cast `/Game/Default/AOESystem/BP_TPSGameState` (`GameplayStatics.GetGameState`)))
    (`/Game/Default/AOESystem/BP_TPSGameState.SpawnAOE` _asbp_tpsgame_state (`self.K2_GetActorLocation`) 400.0 true self (delegate `커스텀이벤트`) 2.5 (struct :`R` 1.0 :`A` 1.0))))

(event `커스텀이벤트`
  (params (`Hit Actor` :type "Actor Object Reference"))
  (message `/Game/Default/AOESystem/BPI_HealthInterface.Damage` `Hit Actor` 100.0))

(fn `GetHealthAsRatio`
  (returns (HealthRatio :type "Float (double-precision)"))
  (return (/ (`self.Health`) (`self.MaxHealth`))))

(fn `UserConstructionScript`
  (`parent.UserConstructionScript`))