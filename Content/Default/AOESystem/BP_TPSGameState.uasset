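; Game State that provides SpawnAOE, a reusable area-of-effect query reporting affected actors through a caller-supplied delegate.
; A sphere overlap gathers Pawns implementing BPI_HealthInterface, excluding the instigator, with optional debug drawing.
; With RequireLOS, an actor counts if any Visibility trace to its bounds center or eight upper/lower edge points hits nothing.
; The delegate is bound only for that call; damage is left to the caller.
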(fn `Get Box Corners`
  (params (Origin :type "Vector Structure") (`Box Extent` :type "Vector Structure"))
  (returns (Corners :type "Array of Vector Structure"))
  (bind (_box_extent_x _box_extent_y _box_extent_z) (`KismetMathLibrary.BreakVector` (`local.Box Extent`)))
  (bind (_box_extent_x_2 _box_extent_y_2 _box_extent_z_2) (`KismetMathLibrary.BreakVector` (`local.Box Extent`)))
  (bind (_box_extent_x_3 _box_extent_y_3 _box_extent_z_3) (`KismetMathLibrary.BreakVector` (`local.Box Extent`)))
  (bind (_box_extent_x_4 _box_extent_y_4 _box_extent_z_4) (`KismetMathLibrary.BreakVector` (`local.Box Extent`)))
  (bind (_box_extent_x_5 _box_extent_y_5 _box_extent_z_5) (`KismetMathLibrary.BreakVector` (`local.Box Extent`)))
  (bind (_box_extent_x_6 _box_extent_y_6 _box_extent_z_6) (`KismetMathLibrary.BreakVector` (`local.Box Extent`)))
  (bind (_box_extent_x_7 _box_extent_y_7 _box_extent_z_7) (`KismetMathLibrary.BreakVector` (`local.Box Extent`)))
  (bind (_box_extent_x_8 _box_extent_y_8 _box_extent_z_8) (`KismetMathLibrary.BreakVector` (`local.Box Extent`)))
  (return (`|MakeArray` (`local.Origin`) (+ (`local.Origin`) (`KismetMathLibrary.MakeVector` _box_extent_x 0.0 _box_extent_z)) (+ (`local.Origin`) (`KismetMathLibrary.MakeVector` (* _box_extent_x_2 -1.0) 0.0 _box_extent_z_2)) (+ (`local.Origin`) (`KismetMathLibrary.MakeVector` 0.0 _box_extent_y_3 _box_extent_z_3)) (+ (`local.Origin`) (`KismetMathLibrary.MakeVector` 0.0 (* _box_extent_x_4 -1.0) _box_extent_z_4)) (+ (`local.Origin`) (`KismetMathLibrary.MakeVector` _box_extent_x_7 0.0 (* _box_extent_z_7 -1.0))) (+ (`local.Origin`) (`KismetMathLibrary.MakeVector` (* _box_extent_x_8 -1.0) 0.0 (* _box_extent_z_8 -1.0))) (+ (`local.Origin`) (`KismetMathLibrary.MakeVector` 0.0 _box_extent_y_6 (* _box_extent_z_6 -1.0))) (+ (`local.Origin`) (`KismetMathLibrary.MakeVector` 0.0 (* _box_extent_x_5 -1.0) (* _box_extent_z_5 -1.0))))))

(fn `SpawnAOE`
  (params (Location :type "Vector Structure") (Radius :type "Float (double-precision)") (`Require LOS` :type Boolean) (`Aoe Instigator` :type "Actor Object Reference") (`Hit Delegate` :type "Delegate (by ref)") (`Draw Debug Duration` :type "Float (double-precision)") (`Debug Color` :type "LinearColor Structure"))
  (locals (`Current Actor` :type "Actor Object Reference"))
  (bind _draw_debug_duration (`local.Draw Debug Duration`))
  (bind _draw_debug_duration_2 (`local.Draw Debug Duration`))
  (bind (_origin _boxextent) (`self.GetActorBounds` (`local.Current Actor`) true true))
  (add `self.AOE Hit Delegate` `Hit Delegate`)
  (`|ExecutionSequence`
    (:`then_0`
      (if (> _draw_debug_duration 0.0)
        (`KismetSystemLibrary.DrawDebugSphere` (`local.Location`) (`local.Radius`) 16 (`local.Debug Color`) _draw_debug_duration))
      (bind _outactors (`KismetSystemLibrary.SphereOverlapActors` (`local.Location`) (`local.Radius`) (`|MakeArray` "ObjectTypeQuery3" :!type "EObjectTypeQuery Enum") "/Script/Engine.Actor" (`|MakeArray` (`local.Aoe Instigator`))))
      (for _array_element _outactors
        (bind _output_get (set `local.Current Actor` _array_element))
        (if (`KismetSystemLibrary.DoesImplementInterface` _output_get "/Game/Default/AOESystem/BPI_HealthInterface.BPI_HealthInterface_C")
          (if (`local.Require LOS`)
            (bind _corners (`self.Get Box Corners` _origin _boxextent))
            (for _array_element_2 _corners
              (bind (_outhit _returnvalue) (`KismetSystemLibrary.LineTraceSingle` (`local.Location`) _array_element_2 "TraceTypeQuery1" false (`|MakeArray` (`local.Aoe Instigator`)) (select `bool` (> _draw_debug_duration_2 0.0) :`true` "ForDuration" :!type "EDrawDebugTrace Enum") true (struct :`R` 1.0 :`A` 1.0) (struct :`G` 1.0 :`A` 1.0) _draw_debug_duration_2))
              (if (not _returnvalue)
                (`self.AOE Hit Delegate` (`local.Current Actor`))
                (break)))
            (else
              (`self.AOE Hit Delegate` (`local.Current Actor`)))))))
    (:`then_1`
      (remove `self.AOE Hit Delegate` `Hit Delegate`))))

(fn `UserConstructionScript`)